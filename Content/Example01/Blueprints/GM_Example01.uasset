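; Game mode for Example01 that spawns and possesses a player character for each joining controller without a pawn.
; On HandleStartingNewPlayer, SpawnMPChar uses the first existing BP_Character_Example01 as the spawn anchor, falling back to the first PlayerStart if none exists.
; It applies a random horizontal offset to that transform and always spawns, adjusting for collisions where possible, then possesses the new character.
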(event `self.HandleStartingNewPlayer`
  (params (NewPlayer :type "PlayerController Object Reference"))
  (`self.SpawnMPChar` NewPlayer))

(fn `SpawnMPChar`
  (params (PlayerControllerRef :type "PlayerController Object Reference"))
  (locals (SpawnTransform :type "Transform Structure") (Local_StoredPlayer :type "Actor Object Reference"))
  (bind (_spawntransform_location _spawntransform_rotation _spawntransform_scale) (`KismetMathLibrary.BreakTransform` (`local.SpawnTransform`)))
  (`/Engine/EditorBlueprintResources/StandardMacros.IsValid` (`Controller.K2_GetPawn` (`local.PlayerControllerRef`))
    (:`Is Valid`
      (return))
    (:`Is Not Valid`
      (set `local.SpawnTransform` (struct))
      (bind _outactors (`GameplayStatics.GetAllActorsOfClass` "/Game/Example01/Blueprints/BP_Character_Example01.BP_Character_Example01_C"))
      (bind _output_get (set `local.Local_StoredPlayer` (`|GetArrayItem` _outactors)))
      (`/Engine/EditorBlueprintResources/StandardMacros.IsValid` _output_get
        (:`Is Valid`
          (set `local.SpawnTransform` (`self.GetTransform` (`local.Local_StoredPlayer`))))
        (:`Is Not Valid`
          (bind _outactors_2 (`GameplayStatics.GetAllActorsOfClass` "/Script/Engine.PlayerStart"))
          (set `local.SpawnTransform` (`self.GetTransform` (`|GetArrayItem` _outactors_2)))))
      (bind _output_get_2 (set `local.SpawnTransform` (`KismetMathLibrary.MakeTransform` (+ _spawntransform_location (`KismetMathLibrary.MakeVector` (select `bool` (`KismetMathLibrary.RandomBool`) :`false` (`KismetMathLibrary.RandomFloatInRange` -50.0 -150.0) :`true` (`KismetMathLibrary.RandomFloatInRange` 50.0 150.0) :!type "Float (double-precision)") (`KismetMathLibrary.RandomFloatInRange` -50.0 -150.0))) _spawntransform_rotation _spawntransform_scale)))
      (bind _returnvalue (`|SpawnActorFromClass` "/Game/Example01/Blueprints/BP_Character_Example01.BP_Character_Example01_C" _output_get_2 "AdjustIfPossibleButAlwaysSpawn" "OverrideRootScale" (`local.PlayerControllerRef`) null))
      (`Controller.Possess` (`local.PlayerControllerRef`) _returnvalue))))

(fn `UserConstructionScript`)